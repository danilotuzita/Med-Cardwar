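; Game manager for a turn-based card duel between the player and an AI, owning HP, turn state and win/loss.
; Played cards are read from a data table and validated against the current side and phase: attack, defense or effect.
; Defense resolves pending damage, while numbered effects add poison, healing or forced skips via ValidatePlay.
; NextPhase flips sides, checks health and fires dispatchers, with poison and heal ticking each turn; ClearAllEffect is an empty stub.
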(event `addRef`
  (params (p :type "/Game/Blueprints/BP_Deck_Manager Object Reference") (a :type "/Game/Blueprints/BP_Deck_Manager Object Reference"))
  (set `self.Player` p)
  (set `self.AI` a))

(event `useCard`
  (params (player :type Boolean) (idCarta :type Integer) (refCard :type "/Game/Blueprints/BP_Card Object Reference"))
  (bind _returnvalue (`|GetDataTableRow` "/Game/data/data_cards.data_cards" (`KismetStringLibrary.Conv_StringToName` (`KismetStringLibrary.Conv_IntToString` idCarta)))
    (:`then`
      (`self.validatePlay` _returnvalue player))))

(event `skipPhase`
  (params (player :type Boolean))
  (if (== player (`self.sideTurn`))
    (`self.validatePlay` (struct) player true)))

(event `self.ReceiveBeginPlay`)

(fn `applyPoison`
  (`|ExecutionSequence`
    (:`then_0`
      (for (_array_element _array_index) (`self.poison`)
        (if _array_element
          (`/Engine/EditorBlueprintResources/StandardMacros.DecrementInt` (select `int` _array_index :`0` (`self.aiHP`) :`1` (`self.playerHP`))))))
    (:`then_1`
      (for (_array_element_2 _array_index_2) (`self.heal`)
        (if _array_element_2
          (`/Engine/EditorBlueprintResources/StandardMacros.IncrementInt` (select `int` _array_index_2 :`0` (`self.aiHP`) :`1` (`self.playerHP`))))))))

(fn `atkPhase`
  (params (dmg :type Integer) (autoDmg :type Integer) (effect :type Integer))
  (`|ExecutionSequence`
    (:`then_0`
      (switch `int` effect
        (:`1`
          (set `self.cantDefend` true))
        (:`2`
          (`|VariableSetRef` (select `bool` (`self.attacking`) :`false` (`self.effect2Ai`) :`true` (`self.effect2Player`)) true))))
    (:`then_1`
      (bind _output_get (set `self.potentialAtkDmg` dmg))
      (bind _output_get_2 (set `self.potentialAutoDmg` (`local.autoDmg`)))
      (`|ExecutionSequence`
        (:`then_0`
          (if (> (+ _output_get_2 _output_get) 0)
            (`GameplayStatics.PlaySound2D` "/Game/Audio/sword.sword" 1.0 1.0 0.0 null null)))
        (:`then_1`
          (`self.nextPhase`)
          ;[1 1 1] efeito 1 - não pode se defender
          (if (`self.cantDefend`)
            (`self.validatePlay` (struct) (not (`self.attacking`)) true)))))))

(fn `calculateDmg`
  (bind _returnvalue (select `bool` (`self.attacking`) :`false` (`self.aiHP`) :`true` (`self.playerHP`)))
  (bind _returnvalue_2 (select `bool` (`self.attacking`) :`false` (`self.playerHP`) :`true` (`self.aiHP`)))
  (`|VariableSetRef` _returnvalue_2 (- _returnvalue_2 (`KismetMathLibrary.Max` (- (`self.potentialAtkDmg`) (`self.potentialDefDmg`)))))
  (`|VariableSetRef` _returnvalue (- _returnvalue (`self.potentialAutoDmg`)))
  (`self.clearPotential`))

(fn `checkHealth`
  (returns (gameEnded :type Boolean))
  (if (and (> (`self.aiHP`) 0) (> (`self.playerHP`) 0))
    (return false)
    (else
      (if (and (<= (`self.playerHP`) 0) (<= (`self.aiHP`) 0))
        (set `self.winner` (select `bool` (`self.attacking`) :`true` 1))
        (else
          (set `self.winner` (select `bool` (> (`self.playerHP`) (`self.aiHP`)) :`true` 1))))
      (return true))))

(fn `clearAllEffect`)

(fn `clearPotential`
  (set `self.potentialAtkDmg` 0)
  (set `self.potentialDefDmg` 0)
  (set `self.potentialAutoDmg` 0)
  (set `self.cantDefend` false))

(fn `defPhase`
  (params (def :type Integer) (dmg :type Integer) (effect :type Integer))
  (bind _output_get (set `self.potentialDefDmg` def))
  (set `self.potentialAutoDmg` (+ dmg (`self.potentialAutoDmg`)))
  (`|ExecutionSequence`
    (:`then_0`
      ;[1 1 1] efeito 13 - rebate 1/2 do ataque
      (if (== (`local.effect`) 13)
        (set `self.potentialAutoDmg` (+ (/ (`self.potentialAtkDmg`) 2) (`self.potentialAutoDmg`)))))
    (:`then_1`
      (if (> _output_get 0)
        (`GameplayStatics.PlaySound2D` "/Game/Audio/shield.shield" 1.0 1.0 0.0 null null)))
    (:`then_2`
      (`self.calculateDmg`)
      (`self.nextPhase`))))

(fn `effect5`
  (bind _output_get (set `self.playerHP` (`KismetMathLibrary.Max` (`self.playerHP`) (`self.aiHP`))))
  (set `self.aiHP` _output_get)
  (`/Game/Blueprints/BP_Deck_Manager.clearHand` (select `bool` (`self.attacking`) :`false` (`self.AI`) :`true` (`self.Player`))))

(fn `effectPhase`
  (params (effect :type Integer) (dmg :type Integer) (autodmg :type Integer))
  (bind _returnvalue (select `bool` (`self.attacking`) :`false` (`self.aiHP`) :`true` (`self.playerHP`)))
  (bind _returnvalue_2 (select `bool` (`self.attacking`) :`false` (`self.playerHP`) :`true` (`self.aiHP`)))
  (`|ExecutionSequence`
    (:`then_0`
      (switch `int` effect
        (:`2`
          (set `self.effect2` true))
        (:`3`
          (`self.clearAllEffect`))
        (:`4`
          ;[1 1 1] set veneno
          (`KismetArrayLibrary.Array_Set` (`self.poison`) (select `bool` (`self.attacking`) :`false` 1) true))
        (:`5`
          (`self.effect5`))
        (:`6`
          ;[1 1 1] efeito 6 - oponente n ataca
          (`|VariableSetRef` (select `bool` (`self.attacking`) :`false` (`self.effect2Player`) :`true` (`self.effect2Ai`)) true))
        (:`10`
          ;[1 1 1] set heal
          (`KismetArrayLibrary.Array_Set` (`self.heal`) (select `bool` (`self.attacking`) :`false` 1) true))
        (:`12`
          (set `self.effect12` true))))
    (:`then_1`
      ;[1 1 1] dano imediato da carta de magia
      (`|VariableSetRef` _returnvalue_2 (- _returnvalue_2 (`local.dmg`)))
      (`|VariableSetRef` _returnvalue (- _returnvalue (`local.autodmg`))))
    (:`then_2`
      (`self.nextPhase`))
    (:`then_3`
      (`|ExecutionSequence`
        (:`then_0`
          (if (`self.effect2`)
            ;[1 1 1] efeito 2 - skipa ataque self
            (if (`self.attacking`)
              (if (`self.effect2Player`)
                (set `self.effect2Player` false)
                (`self.validatePlay` (struct) (`self.attacking`) true :!label _label)
                (set `self.effect2` false))
              (elif (`self.effect2Ai`)
                (set `self.effect2Ai` false)
                (goto _label)))))
        (:`then_1`
          (if (`self.effect12`)
            ;[1 1 1] efeito 12 - seu turno novamente
            (`self.validatePlay` (struct) (`self.attacking`) true)
            (`self.validatePlay` (struct) (not (`self.attacking`)) true)
            (`self.validatePlay` (struct) (`self.attacking`) true)
            (set `self.effect12` false)))))))

(fn `nextPhase`
  (set `self.sideTurn` (not (`self.sideTurn`)))
  (bind _gameended (`self.checkHealth`))
  (if _gameended
    (`self.dispatchGameEnded`)
    (`GameplayStatics.PlaySound2D` (select `int` (`self.winner`) :`0` "/Game/Audio/defeat.defeat" :`1` "/Game/Audio/victory.victory" :!type "SoundBase Object Reference") 1.0 1.0 0.0 null null)
    (else
      (if (>= (`self.turnPhase`) 2)
        (set `self.turnPhase` 0)
        (`self.nextTurn`)
        (else
          (`/Engine/EditorBlueprintResources/StandardMacros.IncrementInt` (`self.turnPhase`)
            (:`  `
              _))))
      (`self.dispatchUpdateTurn`)
      (return))))

(fn `nextTurn`
  (`/Engine/EditorBlueprintResources/StandardMacros.IncrementInt` (`self.turnCount`)
    (:`  `
      (set `self.attacking` (not (`self.attacking`)))
      (`self.applyPoison`)
      (`self.dispatchEndTurnAlert`)
      (return))))

(fn `printPhase`
  (`KismetSystemLibrary.PrintString` (`KismetStringLibrary.Concat_StrStr` "Current Turn: " (`KismetStringLibrary.Conv_IntToString` (`self.turnPhase`)) " - " (select `bool` (`self.sideTurn`) :`false` "AI" :`true` "Player")) true true (struct :`G` 0.66 :`B` 1.0 :`A` 1.0) 5.0))

(fn `UserConstructionScript`)

(fn `validatePlay`
  (params (data :type "/Game/data/structure/datastructure_card Structure") (player :type Boolean) (skip :type Boolean))
  (bind (_classe _nome _descricao _tipo _dano _auto_dano _defesa _efeito) (break `/Game/data/structure/datastructure_card` data))
  (if skip
    (switch `int` (`self.turnPhase`)
      (:`0`
        (`self.atkPhase` 0))
      (:`1`
        (`self.defPhase` 0))
      (:`2`
        (`self.effectPhase` 0)))
    (elif (and (== _tipo (`self.turnPhase`)) (== (`local.player`) (`self.sideTurn`)))
      (switch `int` _tipo
        (:`0`
          (`self.atkPhase` _dano _auto_dano _efeito))
        (:`1`
          (`self.defPhase` _defesa _dano _efeito))
        (:`2`
          (`self.effectPhase` _efeito _dano _auto_dano))))))