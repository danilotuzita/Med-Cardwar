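; Deck and hand manager for one side of a card battle, player or AI, that also shows that side's character flipbook.
; It builds the deck from the saved player deck or character DataTables, reshuffling drawn IDs back when it empties.
; Draws reuse pooled card actors passed in through addReferences.
; The player selects cards or skip via throttled axis input, while the AI steps with delays to a random usable card, or skips.
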(event `self.ReceiveTick`
  (params (DeltaSeconds :type "Float (single-precision)"))
  (if (<= (`KismetArrayLibrary.Array_Length` (`self.deck`)) 0)
    (set `self.deck` (`self.deckDead`))
    (for _ (range (+ (`self.shuffle`) 1))
      (`self.shuffleDeck`))
    (`KismetArrayLibrary.Array_Clear` (`self.deckDead`))))

(event `self.ReceiveBeginPlay`
  (`self.createDeck`)
  (for _ (range (+ (`self.shuffle`) 1))
    (`self.shuffleDeck`)))

(event `endTurn`
  (if (== (`/Game/Blueprints/BP_Game_Manager.attacking` (`self.gameManager`)) (`self.player`))
    (for (_array_element _array_index) (`self.cardsDrawn`)
      (`/Engine/EditorBlueprintResources/StandardMacros.IsValid` _array_element
        (:`Is Not Valid`
          (`KismetSystemLibrary.PrintString` (`KismetStringLibrary.Conv_IntToString` _array_index) true true (struct :`G` 1.0 :`B` 0.127968 :`A` 1.0))
          (`self.pullCard` -1 _array_index)
          (break))))))

(event `endGame`
  (set `self.gameEnded` true)
  (`self.toggleInput` true))

(event `updateTurn`
  (set `self.aiSelectCard` -1)
  (for _array_element (`self.cardsDrawn`)
    (`/Engine/EditorBlueprintResources/StandardMacros.IsValid` _array_element
      (:`Is Valid`
        (`/Game/Blueprints/BP_Card.updateTurn` _array_element))))
  (`/Game/Blueprints/BP_Card.updateTurn` (`self.previewCard`))
  (if (and (not (`/Game/Blueprints/BP_Game_Manager.sideTurn` (`self.gameManager`))) (not (`self.player`)))
    (`self.Think`)))

(event `addReferences`
  (params (player :type Boolean) (previewCard :type "/Game/Blueprints/BP_Card Object Reference") (cards :type "Array of /Game/Blueprints/BP_Card Object Reference") (gameManager :type "/Game/Blueprints/BP_Game_Manager Object Reference") (skipButton :type "/Game/Blueprints/BP_skipPhaseButton Object Reference"))
  ;[1 1 1] Init
  (set `self.skipButton` skipButton)
  (set `self.player` player)
  (set `self.previewCard` previewCard)
  (bind _output_get (set `self.cards` cards))
  (bind _output_get_2 (set `self.gameManager` gameManager))
  (for _array_element _output_get
    (`/Game/Blueprints/BP_Card.makeCard` _array_element (`self.K2_GetActorLocation`) (`self.previewCard`) (`self.player`) _output_get_2))
  (bind _index (`/Engine/EditorBlueprintResources/StandardMacros.ForLoopWithDelay` 0 (`self.startHand`) :!label _label)
    (:`LoopBody`
      (`self.pullCard` _index _index))
    (:`Completed`
      (if (`self.player`)
        (`self.toggleInput` false)
        (set `self.lastActionTime` (`GameplayStatics.GetRealTimeSeconds`)))
      (`self.updateTurn`))
    (:`DelayOut`
      (`KismetSystemLibrary.Delay` (`self.delayToDraw`))
      (goto _label :!via `DelayIn`))))

(event `InputAxis|X-Axis`
  (params (AxisValue :type "Float (single-precision)"))
  (bind _returnvalue (`KismetMathLibrary.FTrunc` AxisValue))
  ;[1 1 1] Input de seleção de carta
  (if (== (`KismetMathLibrary.Abs` AxisValue) 1.0)
    (if (`self.buttonSelected`)
      (`self.selectButton`))
    (if (== _returnvalue (`self.lastAxisDiretion`))
      (if (<= (`self.deltaToInteraction`) (- (`GameplayStatics.GetRealTimeSeconds`) (`self.lastActionTime`)))
        (`self.selectCard` _returnvalue :!label _label_2)
        (set `self.lastActionTime` (`GameplayStatics.GetRealTimeSeconds`))
        (set `self.lastAxisDiretion` _returnvalue))
      (else
        (goto _label_2)))))

(event `InputAxis|Y-Axis`
  (params (AxisValue :type "Float (single-precision)"))
  (bind _returnvalue (`KismetMathLibrary.FTrunc` AxisValue))
  ;[1 1 1] Input de Seleção do botão de pular fase
  (if (== (`KismetMathLibrary.Abs` AxisValue) 1.0)
    (if (== _returnvalue (`self.lastAxisDiretion`))
      (if (<= (`self.deltaToInteraction`) (- (`GameplayStatics.GetRealTimeSeconds`) (`self.lastActionTime`)))
        (`self.selectButton` :!label _label_3)
        (set `self.lastActionTime` (`GameplayStatics.GetRealTimeSeconds`))
        (set `self.lastAxisDiretion` _returnvalue))
      (else
        (goto _label_3)))))

(event `Think`
  (bind _deltatointeraction (`self.deltaToInteraction`))
  ;[1 1 1] Logica da AI
  (if (not (`self.gameEnded`))
    (`KismetSystemLibrary.Delay` 1.0)
    (`self.selectCard` 0)
    (bind _index (`self.aiDecideCard`))
    (bind _output_get (set `self.aiSelectCard` _index))
    (if (< _output_get 0)
      (`self.hidePreviewCard`)
      (`KismetSystemLibrary.Delay` 2.0)
      (`/Game/Blueprints/BP_Game_Manager.skipPhase` (`self.gameManager`) false)
      (else
        (`/Engine/EditorBlueprintResources/StandardMacros.WhileLoopWithDelay` (!= _output_get (`self.selectedCard`)) :!label _label_4
          (:`LoopBody`
            (`self.aiChooseCard` _output_get))
          (:`Completed`
            (`KismetSystemLibrary.Delay` _deltatointeraction)
            (`self.useCard`))
          (:`DelayOut`
            (`KismetSystemLibrary.Delay` _deltatointeraction)
            (goto _label_4 :!via `DelayIn`)))))))

(event `InputAction|Accept`
  (params (Key :type "Key Structure"))
  ;[1 1 1] Input de Aceitar
  (:`Released`
    (if (== (`self.player`) (`/Game/Blueprints/BP_Game_Manager.sideTurn` (`self.gameManager`)))
      (if (`self.buttonSelected`)
        (`/Game/Blueprints/BP_Game_Manager.skipPhase` (`self.gameManager`) true)
        (`self.selectButton`)
        (else
          (`self.useCard`))))))

(event `Key|R`
  (params (Key :type "Key Structure"))
  (:`Pressed`
    (`/Game/Blueprints/BP_Game_Manager.skipPhase` (`self.gameManager`) true)))

(event `Key|E`
  (params (Key :type "Key Structure"))
  (:`Pressed`
    (`/Game/Blueprints/BP_Game_Manager.skipPhase` (`self.gameManager`) false)))

(event `Key|T`
  (params (Key :type "Key Structure"))
  (:`Pressed`
    (`/Game/Blueprints/BP_Game_Manager.printPhase` (`self.gameManager`))))

(event `Key|H`
  (params (Key :type "Key Structure"))
  (:`Pressed`
    (for (_array_element _array_index) (`self.cardsDrawn`)
      (`KismetSystemLibrary.PrintString` (`KismetStringLibrary.Conv_IntToString` _array_index) (`KismetSystemLibrary.IsValid` _array_element) false))))

(event `Key|G`
  (params (Key :type "Key Structure")))

(event `Key|O`
  (params (Key :type "Key Structure"))
  (:`Released`
    (`KismetSystemLibrary.PrintString` (`KismetSystemLibrary.GetDisplayName` (`|GetArrayItem` (`self.cardsDrawn`) (`self.selectedCard`))))))

(event `Key|P`
  (params (Key :type "Key Structure"))
  (:`Released`
    (`self.printHandAI`)))

(fn `addCard`
  (params (id :type Integer) (count :type Integer))
  (for _ (range (+ count 1))
    (`KismetArrayLibrary.Array_Add` (`self.deck`) id)))

(fn `aiChooseCard`
  (params (index :type Integer))
  (if (!= index (`self.selectedCard`))
    (`self.selectCard` (select `bool` (< (`self.selectedCard`) (`local.index`)) :`false` -1 :`true` 1))))

(fn `aiDecideCard`
  (returns (index :type Integer))
  (locals (avaiableCards :type "Array of Integer"))
  (bind _returnvalue (`KismetArrayLibrary.Array_Length` (`local.avaiableCards`)))
  (`KismetArrayLibrary.Array_Clear` (`local.avaiableCards`))
  (for (_array_element _array_index) (`self.cardsDrawn`)
    (`/Engine/EditorBlueprintResources/StandardMacros.IsValid` _array_element
      (:`Is Valid`
        (if (`/Game/Blueprints/BP_Card.canUse` _array_element)
          (`KismetArrayLibrary.Array_Add` (`local.avaiableCards`) _array_index)))))
  (if (<= _returnvalue 0)
    (return -1)
    (else
      (return (`|GetArrayItem` (`local.avaiableCards`) (`KismetMathLibrary.RandomInteger` _returnvalue))))))

(fn `clearHand`
  (bind _cardsdrawn (`self.cardsDrawn`))
  (for (_array_element _array_index) _cardsdrawn
    (`/Game/Blueprints/BP_Card.setOpacity` _array_element 0.0 true)
    (`KismetArrayLibrary.Array_Remove` _cardsdrawn _array_index)
    (`KismetArrayLibrary.Array_Add` _cardsdrawn)))

(fn `createDeck`
  (bind _returnvalue (select `int` (`self.character`) :`0` "/Game/data/knight_deck.knight_deck" :`1` "/Game/data/spy_deck.spy_deck" :`2` "/Game/data/wiz_deck.wiz_deck" :!type "DataTable Object Reference"))
  (if (`self.player`)
    (bind _asbp_game_instance (cast `/Game/Blueprints/BP_GameInstance` (`GameplayStatics.GetGameInstance`)))
    (bind _output_get (set `self.deck` (`/Game/Blueprints/BP_GameInstance.playerDeck` _asbp_game_instance)))
    (if (not (> (`KismetArrayLibrary.Array_Length` _output_get) 0))
      (bind _outrownames (`DataTableFunctionLibrary.GetDataTableRowNames` _returnvalue :!label _label))
      (for _array_element _outrownames
        (bind _returnvalue_2 (`|GetDataTableRow` _returnvalue _array_element)
          (:`then`
            (`self.addCard` (`KismetStringLibrary.Conv_StringToInt` (`KismetStringLibrary.Conv_NameToString` _array_element)) (- (`.count_2_F5A698C44F1D29492A06939014882050` (break `/Game/data/structure/datastructure_deck` _returnvalue_2)) 1)))
          (:`RowNotFound`
            (break)))))
    (else
      (goto _label))))

(fn `getFreeCard`
  (returns (index :type Integer))
  (locals (found :type Boolean))
  (for (_array_element _array_index) (`self.cards`)
    (`|ExecutionSequence`
      (:`then_0`
        (for _array_element_2 (`self.cardsDrawn`)
          (bind _output_get (set `local.found` (`KismetStringLibrary.EqualEqual_StrStr` (`KismetSystemLibrary.GetDisplayName` _array_element_2) (`KismetSystemLibrary.GetDisplayName` _array_element))))
          (if _output_get
            (break))))
      (:`then_1`
        (if (not (`local.found`))
          (return _array_index))))))

(fn `getRandomCopy`
  (params (arraySize :type Integer))
  (returns (index :type Integer) (value :type Integer))
  (bind _returnvalue (`KismetMathLibrary.RandomInteger` arraySize))
  (return _returnvalue (`|GetArrayItem` (`self.deck`) _returnvalue)))

(fn `handleAI`
  (`self.handleCharacter`))

(fn `handleCharacter`
  (`PaperFlipbookComponent.SetFlipbook` (`self.PaperFlipbook`) (`|GetArrayItem` (`self.flipbooks`) (`self.character`)))
  (if (`self.player`)
    (`SceneComponent.SetRelativeScale3D` (`self.PaperFlipbook`) (-1.0 1.0 1.0))))

(fn `handlePlayer`
  (`self.handleCharacter`))

(fn `hidePreviewCard`
  (bind _output (`|GetArrayItem` (`self.cardsDrawn`) (`self.selectedCard`)))
  (`/Game/Blueprints/BP_Card.setOpacity` (`self.previewCard`) 0.0 false)
  (`/Engine/EditorBlueprintResources/StandardMacros.IsValid` _output
    (:`Is Valid`
      (`/Game/Blueprints/BP_Card.setOpacity` _output 1.0 false))))

(fn `popDeck`
  (returns (id :type Integer))
  (locals (ret :type Integer))
  (bind _deck (`self.deck`))
  (bind _returnvalue (`KismetArrayLibrary.Array_LastIndex` _deck))
  (bind _output (`|GetArrayItem` _deck _returnvalue))
  (`KismetArrayLibrary.Array_Add` (`self.deckDead`) _output)
  (`KismetArrayLibrary.Array_Remove` (`self.deck`) _returnvalue)
  (return _output))

(fn `printDeck`
  (params (time :type "Float (double-precision)" :default 5.0))
  (locals (debug :type String))
  (for _array_element (`self.deck`)
    (set `local.debug` (`KismetStringLibrary.Concat_StrStr` (`local.debug`) ", " (`KismetStringLibrary.Conv_IntToString` _array_element))))
  (`KismetSystemLibrary.PrintString` (`local.debug`) true true (struct :`R` 1.0 :`A` 1.0) time))

(fn `printHandAI`
  (for (_array_element _array_index) (`self.cardsDrawn`)
    (`/Engine/EditorBlueprintResources/StandardMacros.IsValid` _array_element
      (:`Is Valid`
        (bind _returnvalue (`|GetDataTableRow` "/Game/data/data_cards.data_cards" (`KismetStringLibrary.Conv_StringToName` (`KismetStringLibrary.Conv_IntToString` (`/Game/Blueprints/BP_Card.id` _array_element))))
          (:`then`
            (bind _returnvalue_2 (`KismetStringLibrary.Conv_IntToString` _array_index))
            (`KismetSystemLibrary.PrintString` (`KismetStringLibrary.Concat_StrStr` _returnvalue_2 " - " (`KismetTextLibrary.Conv_TextToString` (`.nome_9_296A046E40BBEE1010DDB5A023F99358` (break `/Game/data/structure/datastructure_card` _returnvalue)))) true true (struct :`G` 0.66 :`B` 1.0 :`A` 1.0) 10.0))))
      (:`Is Not Valid`
        (`KismetSystemLibrary.PrintString` (`KismetStringLibrary.Concat_StrStr` _returnvalue_2 " - livre") true true (struct :`R` 1.0 :`G` 0.061979 :`B` 0.091826 :`A` 1.0) 10.0)))))

(fn `pullCard`
  (params (cardIndex :type Integer :default -1) (handPositon :type Integer))
  (locals (index :type Integer))
  (bind _handpositon (`local.handPositon`))
  (bind _output (`|GetArrayItem` (`self.cards`) (`local.index`)))
  (if (>= cardIndex 0)
    (set `local.index` (`local.cardIndex`))
    (else
      (bind _index (`self.getFreeCard`))
      (set `local.index` _index)))
  (bind _id (`self.popDeck`))
  (`/Game/Blueprints/BP_Card.DrawCard` _output _id (select `bool` (`self.player`) :`false` (* _handpositon -1) :`true` _handpositon) (`self.cardsOnHandPosition`) (`self.cardsOffset`) (`self.cardsScale`) (0.0 0.0 0.0))
  (`KismetArrayLibrary.Array_Set` (`self.cardsDrawn`) (`local.handPositon`) _output)
  (`GameplayStatics.PlaySound2D` "/Game/Audio/card.card" 0.2 1.0 0.0 null null))

(fn `reorderCards`
  (bind _cardsscale (`self.cardsScale`))
  (bind _cardsdrawn (`self.cardsDrawn`))
  (`|ExecutionSequence`
    (:`then_0`
      ;[1 1 1 1 12] retorna a carta de volta para a posição do deck manager
      (`self.K2_SetActorLocation` (`|GetArrayItem` _cardsdrawn (`self.selectedCard`)) (`self.K2_GetActorLocation`) false false))
    (:`then_1`
      ;[1 1 1 0.4 12] reordena o vetor
      (`KismetArrayLibrary.Array_Remove` _cardsdrawn (`self.selectedCard`)))
    (:`then_2`
      (`KismetArrayLibrary.Array_Add` _cardsdrawn))
    (:`then_3`
      ;[1 1 1 0.4 12] reordena as cartas visualmente
      (for (_array_element _array_index) _cardsdrawn
        (`/Engine/EditorBlueprintResources/StandardMacros.IsValid` _array_element
          (:`Is Valid`
            (`/Game/Blueprints/BP_Card.pullCardToHand` _array_element (`/Game/Blueprints/BP_Card.id` _array_element) (select `bool` (`self.player`) :`false` (* _array_index -1) :`true` _array_index) (`self.cardsOnHandPosition`) (`self.cardsOffset`) _cardsscale (0.0 0.0 0.0) _cardsscale true))))
      (set `self.selectedCard` -1))))

(fn `selectButton`
  (if (`self.buttonSelected`)
    (`/Game/Blueprints/BP_skipPhaseButton.unselect` (`self.skipButton`))
    (`/Engine/EditorBlueprintResources/StandardMacros.IsValid` (`|GetArrayItem` (`self.cardsDrawn`) (`self.selectedCard`))
      (:`Is Valid`
        (`self.selectCard` 0))
      (:`Is Not Valid`
        (set `self.selectedCard` -1)
        (`self.selectCard` 1)))
    (else
      (`/Game/Blueprints/BP_skipPhaseButton.select` (`self.skipButton`))
      (`self.hidePreviewCard`)))
  (set `self.buttonSelected` (not (`self.buttonSelected`))))

(fn `selectCard`
  (params (direction :type Integer) (overrde :type Boolean :default false) (overrideValue :type Integer))
  (bind _returnvalue (+ (`local.direction`) (`self.selectedCard`)))
  (bind _output (`|GetArrayItem` (`self.cardsDrawn`) (`self.selectedCard`)))
  (bind _output_2 (`|GetArrayItem` (`self.cardsDrawn`)))
  (bind _output_3 (`|GetArrayItem` (`self.cardsDrawn`) _returnvalue))
  (if overrde
    (set `self.selectedCard` (`local.overrideValue`))
    (else
      (`/Engine/EditorBlueprintResources/StandardMacros.IsValid` _output
        (:`Is Valid`
          (`/Game/Blueprints/BP_Card.unselect` _output))
        (:`Is Not Valid`
          _))
      (`/Engine/EditorBlueprintResources/StandardMacros.IsValid` _output_3
        (:`Is Valid`
          (`/Game/Blueprints/BP_Card.select` _output_3)
          (set `self.selectedCard` _returnvalue))
        (:`Is Not Valid`
          (if (> (`local.direction`) 0)
            (`/Engine/EditorBlueprintResources/StandardMacros.IsValid` _output_2
              (:`Is Valid`
                (`/Game/Blueprints/BP_Card.select` _output_2)
                (set `self.selectedCard` 0)))
            (else
              (bind (_arrayindex _arrayelement) (`/Engine/EditorBlueprintResources/StandardMacros.ReverseForEachLoop` (`self.cardsDrawn`))
                (:`LoopBody`
                  (`/Engine/EditorBlueprintResources/StandardMacros.IsValid` _arrayelement
                    (:`Is Valid`
                      (set `self.selectedCard` _arrayindex)
                      (`/Game/Blueprints/BP_Card.select` _arrayelement)
                      (return))))
                (:`Completed`
                  (set `self.selectedCard` -1))))))))))

(fn `shuffleDeck`
  (returns (deckOriginal :type "Array of Integer"))
  (locals (Deck_original :type "Array of Integer") (temp :type Integer) (temp_index :type Integer :default 0) (deckLen :type Integer))
  (bind _output_get (set `local.Deck_original` (`self.deck`)))
  (set `local.deckLen` (`KismetArrayLibrary.Array_Length` _output_get))
  (for (_array_element _array_index) (`self.deck`)
    (bind _output_get_2 (set `local.temp_index` (`KismetMathLibrary.RandomInteger` (`local.deckLen`))))
    (set `local.temp` (`|GetArrayItem` (`self.deck`) _output_get_2))
    (`KismetArrayLibrary.Array_Set` (`self.deck`) (`local.temp_index`) _array_element)
    (`KismetArrayLibrary.Array_Set` (`self.deck`) _array_index (`local.temp`)))
  (return (`local.Deck_original`)))

(fn `toggleInput`
  (params (overide :type Boolean) (value :type Boolean))
  (bind _returnvalue (`GameplayStatics.GetPlayerController` 0))
  (bind _returnvalue_2 (`GameplayStatics.GetPlayerController` 0))
  (if (`self.player`)
    (if (`local.overide`)
      (if (`local.value`)
        (`self.EnableInput` _returnvalue)
        (set `self.inputOn` true :!label _label)
        (else
          (`self.DisableInput` _returnvalue)
          (set `self.inputOn` false :!label _label_2)))
      (elif (`self.inputOn`)
        (`self.DisableInput` _returnvalue_2)
        (goto _label_2)
        (else
          (`self.EnableInput` _returnvalue_2)
          (goto _label))))))

(fn `useCard`
  (bind _output (`|GetArrayItem` (`self.cardsDrawn`) (`self.selectedCard`)))
  (`/Engine/EditorBlueprintResources/StandardMacros.IsValid` _output
    (:`Is Valid`
      (bind _valid (`/Game/Blueprints/BP_Card.useCard` _output))
      (if _valid
        (`self.reorderCards`)))))

(fn `UserConstructionScript`
  (if (`self.player`)
    (bind _asbp_game_instance (cast `/Game/Blueprints/BP_GameInstance` (`GameplayStatics.GetGameInstance`))
      (:`then`
        (set `self.character` (`/Game/Blueprints/BP_GameInstance.character` _asbp_game_instance)))
      (:`CastFailed`
        _))
    (else
      (set `self.character` (`KismetMathLibrary.RandomInteger` 2))))
  (`self.handleCharacter`))