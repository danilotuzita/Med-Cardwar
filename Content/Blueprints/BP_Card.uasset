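; Card actor for a turn-based card game, painting its name, type, description and effect symbols from the Data_cards table.
; Timelines animate dealing into hand slots, shake, flip and explode effects, with opacity driven through sprite and text materials.
; A linked PreviewCard shows the selection and plays use animations, flipping first for opponent cards.
; UpdateTurn allows use only on matching side and phase, darkening unusable player cards, and UseCard notifies the GameManager.
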(event `self.ReceiveBeginPlay`)

(event `self.ReceiveTick`
  (params (DeltaSeconds :type "Float (single-precision)")))

(event `DrawCard`
  (params (id :type Integer) (handPosition :type Integer) (position :type "Vector Structure") (offset :type "Float (double-precision)") (scale :type "Float (double-precision)") (previousPosition :type "Vector Structure"))
  (`self.paintCard` id true)
  (bind _futurepos (`self.calcFuturePosition` handPosition position offset scale))
  (set `self.futurePosition` _futurepos)
  (`self.SetActorScale3D` (`KismetMathLibrary.MakeVector` scale scale scale))
  (if (== previousPosition (0.0 0.0 0.0))
    (set `self.originalPosition` (`self.K2_GetActorLocation`))
    (bind (_direction _alpha) (`Timeline|Swipe` :!via `PlayFromStart` :!label _label)
      (:`Update`
        (`self.K2_SetActorLocation` (`KismetMathLibrary.VLerp` (`self.originalPosition`) (`self.futurePosition`) _alpha))
        (if (`self.player`)
          (`self.setOpacity` _alpha)
          (else
            (`self.opacitySprite` (`self.card_frame`) _alpha)
            (`self.opacitySprite` (`self.card_back`) _alpha)))))
    (else
      (set `self.originalPosition` previousPosition)
      (goto _label :!via `PlayFromStart`))))

(event `pullCardToHand`
  (params (id :type Integer) (handPosition :type Integer) (position :type "Vector Structure") (offset :type "Float (double-precision)") (scale :type "Float (double-precision)") (previousPosition :type "Vector Structure") (previousScale :type "Float (double-precision)") (justMove :type Boolean))
  (`self.paintCard` id (not justMove))
  (bind _futurepos (`self.calcFuturePosition` handPosition position offset scale))
  (set `self.futurePosition` _futurepos)
  (`self.setOpacity` 1.0)
  (if (== previousPosition (0.0 0.0 0.0))
    (set `self.originalPosition` (`self.K2_GetActorLocation`))
    (bind (_direction _alpha) (`Timeline|Swipe2` :!via `PlayFromStart` :!label _label_2)
      (:`Update`
        (`self.K2_SetActorLocation` (`KismetMathLibrary.VLerp` (`self.originalPosition`) (`self.futurePosition`) _alpha))
        (bind _returnvalue (+ (* _alpha (- scale previousScale)) previousScale))
        (`self.SetActorScale3D` (`KismetMathLibrary.MakeVector` _returnvalue _returnvalue _returnvalue))))
    (else
      (set `self.originalPosition` previousPosition)
      (goto _label_2 :!via `PlayFromStart`))))

(event `cantUseAnim`
  (params (maxAngle :type "Float (double-precision)" :default 15.0) (shakes :type Integer :default 2))
  (`/Engine/EditorBlueprintResources/StandardMacros.ForLoopWithDelay` 1 shakes :!label _label_3
    (:`LoopBody`
      (bind (_direction _shakeness) (`Timeline|shake` :!via `PlayFromStart`)
        (:`Update`
          (`self.K2_SetActorRotation` (`KismetMathLibrary.MakeRotator` 0.0 (* _shakeness maxAngle))))))
    (:`Completed`
      (`self.K2_SetActorRotation` (struct)))
    (:`DelayOut`
      (`KismetSystemLibrary.Delay` 0.25)
      (goto _label_3 :!via `DelayIn`))))

(event `useCardAnim`
  (bind _previewcard (`self.previewCard`))
  (if (`self.player`)
    (bind (_direction _size _opacity) (`Timeline|explode` :!via `PlayFromStart` :!label _label_4)
      (:`Update`
        (`self.SetActorRelativeScale3D` (`self.previewCard`) (`KismetMathLibrary.MakeVector` _size _size _size))
        (`self.setOpacity` (`self.previewCard`) _opacity true))
      (:`Finished`
        (`self.setOpacity` (`self.previewCard`) 0.0 true)))
    (else
      (`self.setOpacity` _previewcard 1.0 true)
      (`self.K2_SetActorRotation` _previewcard (struct :`Yaw` -180.0) false)
      (bind (_direction_2 _rotation) (`Timeline|flipCard` :!via `PlayFromStart`)
        (:`Update`
          (`self.rotateCard` (`self.previewCard`) _rotation))
        (:`Finished`
          (`KismetSystemLibrary.Delay` 1.0)
          (goto _label_4 :!via `PlayFromStart`))))))

(fn `breakString`
  (params (str :type String) (alreadyCut :type String) (max :type Integer))
  (returns (cutString :type String))
  (bind _str (`local.str`))
  (bind _max (`local.max`))
  (bind (_lefts _rights) (`KismetStringLibrary.Split` (`KismetStringLibrary.GetSubstring` (`local.str`) 0 (`local.max`)) " " "IgnoreCase" "FromEnd"))
  (if (> (`KismetStringLibrary.Len` str) max)
    (bind _cutstring (`self.breakString` (`KismetStringLibrary.Concat_StrStr` _rights (`KismetStringLibrary.GetSubstring` _str _max (- (`KismetStringLibrary.Len` _str) _max))) (`KismetStringLibrary.Concat_StrStr` (`local.alreadyCut`) "<br>" _lefts) (`local.max`)))
    (return _cutstring)
    (else
      (return (`KismetStringLibrary.Concat_StrStr` (`local.alreadyCut`) "<br>" (`local.str`))))))

(fn `calcFuturePosition`
  (params (handPosition :type Integer) (position :type "Vector Structure") (offset :type "Float (double-precision)") (scale :type "Float (double-precision)"))
  (returns (futurePos :type "Vector Structure"))
  (bind _card_frame (`self.card_frame`))
  (bind _x (.x (`SceneComponent.K2_GetComponentScale` _card_frame)))
  (return (`KismetMathLibrary.MakeVector` (+ (* (`local.handPosition`) (+ (`local.offset`) (* 2 (* (+ (- (select `bool` (<= _x 0.0) :`false` 1.0 :`true` -1.0 :!type "Float (single-precision)") _x) (`local.scale`)) (.x (`.BoxExtent` (`KismetSystemLibrary.GetComponentBounds` _card_frame))))))) (.x (`local.position`))) (.y (`local.position`)) (.z (`local.position`)))))

(fn `destroySprites`
  (for _array_element (`|MakeArray` (`self.fig`) (`self.card_name_back`) (`self.card_name_frame`))
    (`KismetArrayLibrary.Array_RemoveItem` (`self.sprites`) _array_element)
    (`KismetArrayLibrary.Array_Add` (`self.hiddenSprites`) _array_element)))

(fn `dmgString`
  (params (count :type Integer) (char :type String :default "#") (max :type Integer :default 3))
  (returns (string :type String))
  (locals (temp :type String))
  (if (< count 1)
    (return "")
    (elif (> (`local.count`) (`local.max`))
      (return (`KismetStringLibrary.Concat_StrStr` (`KismetStringLibrary.Conv_IntToString` (`local.count`)) (`local.char`)))
      (else
        (for _ (range (+ (`local.count`) 1))
          (set `local.temp` (`KismetStringLibrary.Concat_StrStr` (`local.temp`) (`local.char`))))
        (return (`local.temp`))))))

(fn `makeCard`
  (params (spawnPosition :type "Vector Structure") (inPreviewCard :type "/Game/Blueprints/BP_Card Object Reference") (inPlayer :type Boolean) (game :type "/Game/Blueprints/BP_Game_Manager Object Reference"))
  (bind _previewcard (`self.previewCard`))
  (bind _game (`local.game`))
  (`|ExecutionSequence`
    (:`then_0`
      (`self.K2_SetActorLocation` (`local.spawnPosition`)))
    (:`then_1`
      (bind _output_get (set `self.previewCard` (`local.inPreviewCard`)))
      (`|ExecutionSequence`
        (:`then_0`
          (set `/Game/Blueprints/BP_Card.player` (`local.inPlayer`) _output_get))
        (:`then_1`
          (set `/Game/Blueprints/BP_Card.gameManager` _game _output_get))
        (:`then_2`
          (set `self.gameManager` _game))))
    (:`then_2`
      (bind _output_get_2 (set `self.player` (`local.inPlayer`)))
      (if _output_get_2
        _))
    (:`then_3`
      (set `self.previewScale` (.x (`self.GetActorScale3D` _previewcard)))
      (set `self.previewPos` (`self.K2_GetActorLocation` _previewcard)))))

(fn `opacitySprite`
  (params (sprite :type "PaperSpriteComponent Object Reference") (opacity :type "Float (double-precision)"))
  (`MeshComponent.SetScalarParameterValueOnMaterials` sprite "Alpha" opacity))

(fn `opacityText`
  (params (opacity :type "Float (double-precision)" :default 0.0))
  (`MaterialInstanceDynamic.SetScalarParameterValue` (`self.textMaterial`) "opacity" opacity))

(fn `paintCard`
  (params (id :type Integer) (paint :type Boolean))
  (bind _output_get (set `self.id` id))
  (if paint
    (bind _returnvalue (`|GetDataTableRow` "/Game/data/data_cards.data_cards" (`KismetStringLibrary.Conv_StringToName` (`KismetStringLibrary.Conv_IntToString` _output_get)))
      (:`then`
        (`|ExecutionSequence`
          (:`then_0`
            (bind (_classe _nome _descricao _tipo _dano _auto_dano _defesa _efeito _fig_tex) (break `/Game/data/structure/datastructure_card` _returnvalue))
            (`self.setName` _nome))
          (:`then_1`
            (`self.setDesc` _descricao))
          (:`then_2`
            (`self.setType` _tipo))
          (:`then_3`
            (`self.setDmg` _dano _auto_dano _defesa))
          (:`then_4`
            (`self.setFig` _fig_tex)))))))

(fn `resetTransludency`
  (for _array_element (`self.sprites`)
    (`PrimitiveComponent.SetTranslucentSortPriority` _array_element (`KismetMathLibrary.FTrunc` (.y (`SceneComponent.K2_GetComponentLocation` _array_element)))))
  (for _array_element_2 (`self.texts`)
    (`PrimitiveComponent.SetTranslucentSortPriority` _array_element_2 (`KismetMathLibrary.FTrunc` (.y (`SceneComponent.K2_GetComponentLocation` _array_element_2))))))

(fn `rotateCard`
  (params (rotation :type "Float (double-precision)"))
  (`self.K2_SetActorRotation` (`KismetMathLibrary.MakeRotator` 0.0 0.0 rotation))
  (`self.resetTransludency`))

(fn `select`
  (bind _previewcard (`self.previewCard`))
  (`self.setOpacity` 0.0)
  (`self.pullCardToHand` _previewcard (`self.id`) 0 (`self.previewPos`) 0.0 (`self.previewScale`) (`self.K2_GetActorLocation`) (.x (`self.GetActorScale3D`)) false)
  (set `self.isSelected` true)
  (`self.updateTurn` _previewcard))

(fn `setDarkness`
  (params (percentage :type "Float (double-precision)"))
  (bind _percentage (`local.percentage`))
  (for (_ _array_index) (`self.sprites`)
    (`MeshComponent.SetVectorParameterValueOnMaterials` (`|GetArrayItem` (`self.sprites`) _array_index) "Color" (`KismetMathLibrary.Conv_LinearColorToVector` (`KismetMathLibrary.MakeColor` _percentage _percentage _percentage)))))

(fn `setDesc`
  (params (desc :type Text))
  (locals (string :type String))
  (bind _cutstring (`self.breakString` (`KismetTextLibrary.Conv_TextToString` desc) "" 20))
  (`TextRenderComponent.K2_SetText` (`self.text_description`) (`KismetTextLibrary.Conv_StringToText` _cutstring)))

(fn `setDmg`
  (params (dmg :type Integer) (autodmg :type Integer) (def :type Integer))
  (locals (text :type String))
  (`|ExecutionSequence`
    (:`then_0`
      (bind _string (`self.dmgString` dmg "#" 2))
      (set `local.text` (`KismetStringLibrary.Concat_StrStr` (`local.text`) _string)))
    (:`then_1`
      (bind _string_2 (`self.dmgString` autodmg "@" 2))
      (set `local.text` (`KismetStringLibrary.Concat_StrStr` (`local.text`) _string_2)))
    (:`then_2`
      (bind _string_3 (`self.dmgString` def "$" 2))
      (set `local.text` (`KismetStringLibrary.Concat_StrStr` (`local.text`) _string_3)))
    (:`then_3`
      (`TextRenderComponent.K2_SetText` (`self.text_effects`) (`KismetTextLibrary.Conv_StringToText` (`local.text`))))))

(fn `setFig`
  (params (fig :type "PaperSprite Object Reference"))
  (`PaperSpriteComponent.SetSprite` (`self.fig`) fig))

(fn `setName`
  (params (name :type Text))
  (`TextRenderComponent.K2_SetText` (`self.text_card_name`) name))

(fn `setOpacity`
  (params (opacity :type "Float (double-precision)") (override :type Boolean))
  (for _array_element (`self.sprites`)
    (`self.opacitySprite` _array_element (`local.opacity`)))
  (if (or (`local.override`) (`self.player`))
    (`self.opacityText` (`local.opacity`))))

(fn `setOpacityHidden`
  (params (opacity :type "Float (double-precision)") (override :type Boolean))
  (for _array_element (`self.hiddenSprites`)
    (`self.opacitySprite` _array_element (`local.opacity`))
    (`self.K2_SetActorRotation` (struct :`Yaw` 180.0 :`Roll` -180.0)))
  (`self.opacityText` (`local.opacity`)))

(fn `setType`
  (params (type :type Integer))
  (`TextRenderComponent.K2_SetText` (`self.text_type`) (select `int` (`local.type`) :`0` "Ataque" :`1` "Defesa" :`2` "Magia")))

(fn `unselect`
  (`self.setOpacity` 1.0)
  (set `self.isSelected` false))

(fn `updateTurn`
  (returns (canUse :type Boolean))
  (bind _gamemanager (`self.gameManager`))
  (bind _returnvalue (`|GetDataTableRow` "/Game/data/data_cards.data_cards" (`KismetStringLibrary.Conv_StringToName` (`KismetStringLibrary.Conv_IntToString` (`self.id`))))
    (:`then`
      (if (`self.player`)
        (bind _returnvalue_2 (and (== (`.tipo_13_7FFAF55C4F8A01774F52FC8A56AFCEF0` (break `/Game/data/structure/datastructure_card` _returnvalue)) (`/Game/Blueprints/BP_Game_Manager.turnPhase` _gamemanager)) (== (`/Game/Blueprints/BP_Game_Manager.sideTurn` _gamemanager) (`self.player`))))
        (if _returnvalue_2
          (`self.setDarkness` 1.0) ; Lighten
          (else
            (`self.setDarkness` 0.4) ; Darken
          )))
      (bind _output_get (set `self.canUse` _returnvalue_2))
      (return _output_get))))

(fn `useCard`
  (returns (valid :type Boolean))
  (if (`self.canUse`)
    (`/Game/Blueprints/BP_Game_Manager.useCard` (`self.gameManager`) (`self.player`) (`self.id`) self)
    (`self.useCardAnim`)
    (return true)
    (else
      (`self.cantUseAnim` (`self.previewCard`) 15.0 2)
      (bind _returnvalue (`|GetDataTableRow` "/Game/data/data_cards.data_cards" (`KismetStringLibrary.Conv_StringToName` (`KismetStringLibrary.Conv_IntToString` (`self.id`))))
        (:`then`
          (return false))))))

(fn `UserConstructionScript`
  (`|ExecutionSequence`
    (:`then_0`
      (set `self.sprites` (`|MakeArray` (`self.fig`) (`self.card_name_frame`) (`self.card_name_back`) (`self.card_back`) (`self.card_frame`))))
    (:`then_1`
      (bind _output_get (set `self.texts` (`|MakeArray` (`self.text_effects`) (`self.text_description`) (`self.text_type`) (`self.text_card_name`))))
      (bind _returnvalue (`KismetMaterialLibrary.CreateDynamicMaterialInstance` "/Game/Materials/MAT_font_pixel.MAT_font_pixel"))
      (for _array_element _output_get
        (`PrimitiveComponent.SetMaterial` _array_element 0 _returnvalue))
      (bind _output_get_2 (set `self.textMaterial` _returnvalue))
      (`MaterialInstanceDynamic.SetVectorParameterValue` :`self` _output_get_2 :`ParameterName` "Color"))
    (:`then_2`
      (`self.setOpacity` 0.0 true)
      (`self.resetTransludency`))))